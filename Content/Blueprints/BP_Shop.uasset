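; BP_Shop is a placeable shop that offers its SpellsToSell list through a WBP_ShopUI widget.
; On BeginPlay it creates the widget and initializes it with that list.
; When the player's controlled pawn enters the Box trigger, it shows the UI and mouse cursor, switches to Game and UI input, and sets IsInShop on the controller.
; Leaving the box reverses all of this.
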(event OnComponentBeginOverlap(Box)
  (params (OverlappedComponent :type Primitive%20Component%20Object%20Reference) (OtherActor :type Actor%20Object%20Reference) (OtherComp :type Primitive%20Component%20Object%20Reference) (OtherBodyIndex :type Integer) (bFromSweep :type Boolean) (SweepResult :type Hit%20Result%20Structure%20%28by%20ref%29))
  (bind _myplayercontroller (CallFunction|GetMyPlayerController))
  (if (== OtherActor (Variables|/Game/Blueprints/BP_MyPlayerController.BP_MyPlayerController_C|GetControlledPawnAsTP _myplayercontroller))
    (UserInterface|Viewport|AddtoViewport (Variables|Default|GetShopUI) 0)
    (Variables|/Script/Engine.PlayerController|SetbShowMouseCursor _myplayercontroller true)
    (Input|SetInputModeGameandUI _myplayercontroller 0 "DoNotLock" false)
    (Variables|/Game/Blueprints/BP_MyPlayerController.BP_MyPlayerController_C|SetisInShop _myplayercontroller true)))

(event OnComponentEndOverlap(Box)
  (params (OverlappedComponent :type Primitive%20Component%20Object%20Reference) (OtherActor :type Actor%20Object%20Reference) (OtherComp :type Primitive%20Component%20Object%20Reference) (OtherBodyIndex :type Integer))
  (bind _myplayercontroller (CallFunction|GetMyPlayerController))
  (if (== OtherActor (Variables|/Game/Blueprints/BP_MyPlayerController.BP_MyPlayerController_C|GetControlledPawnAsTP _myplayercontroller))
    (Widget|RemovefromParent (Variables|Default|GetShopUI))
    (Variables|/Script/Engine.PlayerController|SetbShowMouseCursor _myplayercontroller false)
    (Input|SetInputModeGameOnly _myplayercontroller)
    (Variables|/Game/Blueprints/BP_MyPlayerController.BP_MyPlayerController_C|SetisInShop _myplayercontroller false)))

(event EventBeginPlay
  (bind _returnvalue (UserInterface|CreateWidget "/Game/Blueprints/UI/WBP_ShopUI.WBP_ShopUI_C"))
  (bind _output_get (Variables|Default|SetShopUI _returnvalue))
  (Default|Initialize _output_get (Variables|Default|GetSpellsToSell)))

(fn ConstructionScript)