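; Player controller that manages HP, mana, gold and an inventory of data-asset spells, starting the player with a simple teleport.
; It creates the HUD and a spell-selection widget, pushing stat and icon changes to them and blocking selection while shopping.
; Holding CastSpell on a throwable draws a debug predicted arc each Tick.
; Release calls the spell's CastSpell and, on success, launches a physics-driven BP_ThrowableSpell from the pawn's throw point.
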(event Custom|ChangeHP
  (params (Amount :type Integer))
  (bind _maxhp (Variables|Default|GetMaxHP))
  (bind _output_get (Variables|Default|SetHP (Math|Integer|Clamp(Integer) (+ Amount (Variables|Default|GetHP)) 0 _maxhp)))
  (Default|UpdateHPDisplay (Variables|Default|GetGeneralUI) _output_get _maxhp))

(event Custom|ChangeMana
  (params (Amount :type Integer))
  (bind _maxmana (Variables|Default|GetMaxMana))
  (bind _output_get (Variables|Default|SetMana (Math|Integer|Clamp(Integer) (+ Amount (Variables|Default|GetMana)) 0 _maxmana)))
  (Default|UpdateManaDisplay (Variables|Default|GetGeneralUI) _output_get _maxmana))

(event Custom|AddSpell
  (params (Spell :type BP%20DA%20Spell%20Object%20Reference))
  (Utilities|Array|Add (Variables|Default|GetAvailableSpells) Spell)
  (Default|AddSpell (Variables|Default|GetSpellUI) Spell))

(event Custom|ResetMana
  (bind _maxmana (Variables|Default|GetMaxMana))
  (bind _output_get (Variables|Default|SetMana _maxmana))
  (Default|UpdateManaDisplay (Variables|Default|GetGeneralUI) _output_get _maxmana))

(event Custom|ResetHP
  (bind _maxhp (Variables|Default|GetMaxHP))
  (bind _output_get (Variables|Default|SetHP _maxhp))
  (Default|UpdateHPDisplay (Variables|Default|GetGeneralUI) _output_get _maxhp))

(event Custom|ChangeGold
  (params (Amount :type Integer))
  (bind _output_get (Variables|Default|SetGold (+ Amount (Variables|Default|GetGold))))
  (Default|UpdateGoldDisplay (Variables|Default|GetGeneralUI) _output_get))

(event Custom|ResetGold
  (bind _output_get (Variables|Default|SetGold 1000))
  (Default|UpdateGoldDisplay (Variables|Default|GetGeneralUI) _output_get))

(event Custom|SetCurrentSpell
  (params (Spell :type BP%20DA%20Spell%20Object%20Reference))
  (if (CallFunction|CheckSpellAvailability Spell)
    (bind _output_get (Variables|Default|SetCurrentSpell Spell))
    (Default|UpdateIcon (Variables|Default|GetGeneralUI) (Variables|/Game/Blueprints/SpellBlueprints/BP_DA_Spell.BP_DA_Spell_C|GetSpellIcon _output_get))))

(event Custom|ExitSpellSelection
  (Variables|Default|SetbShowMouseCursor false)
  (Widget|RemovefromParent (Variables|Default|GetSpellUI))
  (Input|SetInputModeGameOnly self))

(event Custom|ChangePlayerSize
  (params (SizeMultiplicator :type Float%20%28single-precision%29))
  (Transformation|SetActorScale3D (Variables|Default|GetControlledPawnAsTP) (* (Math|Vector|MakeVector 1.0 1.0 1.0) SizeMultiplicator)))

(event Custom|ResetPlayerSize
  (params (Duration :type Float%20%28single-precision%29))
  (Utilities|FlowControl|Delay Duration)
  (CallFunction|ChangePlayerSize 1.0))

(event EventBeginPlay
  (Utilities|FlowControl|Sequence
    (:then_0
      (|CreateAndDisplayUI))
    (:then_1
      (CallFunction|ResetHP)
      (CallFunction|ResetMana)
      (CallFunction|ResetGold))
    (:then_2
      (bind _asbp_third_person_character (Utilities|Casting|CastToBP_ThirdPersonCharacter (Pawn|GetControlledPawn)))
      (Variables|Default|SetControlledPawnAsTP _asbp_third_person_character))
    (:then_3
      (CallFunction|AddSpell "/Game/Data/Spells/DA_S_T_SimpleTeleport.DA_S_T_SimpleTeleport"))))

(event EventTick
  (params (DeltaSeconds :type Float%20%28single-precision%29))
  (bind _controlledpawnastp (Variables|Default|GetControlledPawnAsTP))
  (bind _throwablespellref (Variables|/Game/BaseContent/ThirdPersonBP/Blueprints/ThirdPersonCharacter.ThirdPersonCharacter_C|GetThrowableSpellRef _controlledpawnastp))
  (bind _returnvalue (Transformation|GetWorldLocation _throwablespellref))
  (if (Variables|Default|GetisAiming)
    (Class|GameplayStatics|BlueprintPredictProjectilePathAdvanced (Utilities|Struct|MakePredictProjectilePathParams _returnvalue (* (Math|Vector|GetUnitDirection(Vector) (Transformation|GetActorLocation (Variables|Default|GetControlledPawnAsTP)) _returnvalue) (Variables|Default|GetThrowingSpeed)) false 0.0 3.0 true "ECC_WorldStatic" "ObjectTypeQuery1" 0 2e+01 0.0 "ForOneFrame" 1.0 false))))

(event Input|ActionEvents|InputActionCastSpell
  (params (Key :type Key%20Structure :default "None"))
  (:Pressed
    (Utilities|Casting|CastToBP_DA_Spell_Throwable (Variables|Default|GetCurrentSpell))
    (Variables|Default|SetisAiming true))
  (:Released
    (Utilities|FlowControl|Sequence
      (:then_0
        (bind _spellcasted (Default|CastSpell (Variables|Default|GetCurrentSpell) self)))
      (:then_1
        (Variables|Default|SetisAiming false)
        (if _spellcasted
          (|SpawnandThrowThrowablespell))))))

(event Input|ActionEvents|InputActionSpellSelection
  (params (Key :type Key%20Structure :default "None"))
  (:Pressed
    (if (not (Variables|Default|GetisInShop))
      (Variables|Default|SetbShowMouseCursor true)
      (UserInterface|Viewport|AddtoViewport (Variables|Default|GetSpellUI) 0)
      (Input|SetInputModeGameandUI self 0 "DoNotLock" true))))

(fn ConstructionScript)

(fn CheckSpellAvailability
  (params (Spell :type BP%20DA%20Spell%20Object%20Reference))
  (for _array_element (Variables|Default|GetAvailableSpells)
    (if (== _array_element Spell)
      (LocalVariables|SetIsAvailable true)))
  (return (LocalVariables|GetIsAvailable)))