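; Base spell Blueprint that handles mana-gated casting, with an empty ActionOnSpellCast hook for the spell's effect.
; CastSpell stores the passed PlayerController and compares its Mana to ManaCost.
; With enough mana, it deducts the cost through ChangeMana and then calls the hook.
; Either outcome prints a message and returns a success flag to the caller.
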(fn ActiononSpellCast)

(fn CastSpell
  (params (Player%20Controller :type BP%20My%20Player%20Controller%20Object%20Reference))
  (bind _output_get (Variables|Default|SetPlayer%20Controller Player%20Controller))
  (if (>= (Variables|/Game/Blueprints/BP_MyPlayerController.BP_MyPlayerController_C|GetMana _output_get) (Variables|Default|GetManaCost))
    (Default|ChangeMana _output_get (* (Variables|Default|GetManaCost) -1))
    (CallFunction|ActiononSpellCast)
    (Development|PrintString 0 "Spell casted")
    (LocalVariables|SetSpellSuccessfullyCasted true)
    (else
      (Development|PrintString 0 "Not enough mana")
      (LocalVariables|SetSpellSuccessfullyCasted false)))
  (return (LocalVariables|GetSpellSuccessfullyCasted)))