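; BP_ThrowableSpell is a thrown spell projectile whose impact behavior comes from a spell data asset.
; On the first hit of its collision component, it hands the hit actor and itself to the data asset's OnCollision.
; It then spawns the asset's effect at the collision point, deactivates the emitter after a short delay and destroys itself.
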(event OnComponentHit(Collision)
  (params (HitComponent :type Primitive%20Component%20Object%20Reference) (OtherActor :type Actor%20Object%20Reference) (OtherComp :type Primitive%20Component%20Object%20Reference) (NormalImpulse :type Vector :default "0, 0, 0") (Hit :type Hit%20Result%20Structure%20%28by%20ref%29))
  (bind _self self)
  (Utilities|FlowControl|DoOnce false
    (:Completed
      (Default|OnCollision (Variables|Default|GetSpellDataAsset) OtherActor _self)
      (bind _returnvalue (Effects|SpawnEmitteratLocation (Variables|/Game/Blueprints/SpellBlueprints/BP_DA_Spell.BP_DA_Spell_C|GetEffect (Variables|Default|GetSpellDataAsset)) (Transformation|GetWorldLocation (Variables|Default|GetCollision _self))))
      (Utilities|FlowControl|Delay 0.5)
      (Components|Activation|Deactivate _returnvalue)
      (Actor|DestroyActor))))

(event EventBeginPlay)

(fn ConstructionScript)