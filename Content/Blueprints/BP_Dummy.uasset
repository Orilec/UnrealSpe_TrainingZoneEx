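; BP_Dummy is a damageable dummy actor that takes damage over time from spells and displays its HP as text.
; OnDamaged spawns the spell's effect at the dummy and enables Tick for the spell's damage duration, then disables it and deactivates the effect.
; Tick subtracts the per-second damage value every frame without delta-time scaling, clamps HP between zero and MaxHp, and updates the text.
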(event Custom|OnDamaged
  (params (DamageSpell :type BP%20DA%20Spell%20T%20Elemental%20Damages%20Object%20Reference))
  (bind _returnvalue (Effects|SpawnEmitteratLocation (Variables|/Game/Blueprints/SpellBlueprints/BP_DA_Spell.BP_DA_Spell_C|GetEffect DamageSpell) (Transformation|GetWorldLocation (Variables|Default|GetDefaultSceneRoot))))
  (Actor|Tick|SetActorTickEnabled true)
  (Utilities|FlowControl|Delay (Variables|/Game/Blueprints/SpellBlueprints/BP_DA_Spell_T_ElementalDamages.BP_DA_Spell_T_ElementalDamages_C|GetDamagesDuration DamageSpell))
  (Actor|Tick|SetActorTickEnabled false)
  (Components|Activation|Deactivate _returnvalue))

(event Custom|LoseHp
  (params (HP :type Integer))
  (Variables|Default|SetHp (Math|Integer|Clamp(Integer) (- (Variables|Default|GetHp) HP) 0 (Variables|Default|GetMaxHp))))

(event EventTick
  (params (DeltaSeconds :type Float%20%28single-precision%29))
  (CallFunction|LoseHp (Variables|/Game/Blueprints/SpellBlueprints/BP_DA_Spell_T_ElementalDamages.BP_DA_Spell_T_ElementalDamages_C|GetDamagesPerSecond (stale Custom|OnDamaged DamageSpell)))
  (Rendering|Components|TextRender|SetText (Variables|Default|GetTextRender) (Utilities|Text|ToText(Integer) (Variables|Default|GetHp))))

(fn ConstructionScript)